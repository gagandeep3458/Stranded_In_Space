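; BP_Body is a celestial body in a gravity simulation game, becoming a rocket when its name contains "Player".
; SetCurrentForceCPP integrates supplied force into velocity, moving and yawing it; the AddForce path consuming thruster input never runs.
; Tick draws optional velocity readouts, orbits any TargetActor and checks camera bounds for destruction.
; Sun or obstacle hits destroy it, deregistering from BP_Simulator; winning freezes physics, and a timeline fades it into wormholes.
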(event OnComponentHit(Sphere)
  (params (HitComponent :type Primitive%20Component%20Object%20Reference) (OtherActor :type Actor%20Object%20Reference) (OtherComp :type Primitive%20Component%20Object%20Reference) (NormalImpulse :type Vector :default "0, 0, 0") (Hit :type Hit%20Result%20Structure%20%28by%20ref%29))
  ;[0.15 0.15 0.15 0.5] Hit Detection
  (Utilities|IsValid OtherActor
    (:Is%20Valid
      (if (or (Actor|ActorHasTag OtherActor "sun") (Actor|ActorHasTag OtherActor "obstacle"))
        (Utilities|FlowControl|DoOnce false
          (:Completed
            (CallFunction|DestroyBody)
            (Niagara|SpawnSystematLocation "/Game/FX/FX_PlanetDestroyed.FX_PlanetDestroyed" (.Location (Collision|BreakHitResult Hit)))))))))

(event Custom|FadeBodyColor
  (params (WormHole :type BP%20Final%20Wormhole%20Object%20Reference))
  ;[0.15 0.15 0.15 0.5] Fade Body Color
  (bind _opacity (Timeline|ScaleOpacity Play)
    (:Update
      (Rendering|Material|SetScalarParameterValue (Variables|Default|GetDynMaterialInst) "Opacity" _opacity :!class /Script/Engine.MaterialInstanceDynamic)
      (Transformation|SetWorldScale3D (Variables|Default|GetSphere) (Math|Conversions|ToVector(Float) (Math|Float|Lerp (Math|Float|MakeLiteralFloat 0.1) (Math|Float|MakeLiteralFloat 0.75) _opacity))))
    (:Finished
      (Default|FadeWormHole WormHole))))

(event Custom|DestroyBody
  ;[0.15 0.15 0.15 0.5] Destruction
  (Default|RemoveBody (Variables|Default|GetBP_Simulator) self)
  (Actor|DestroyActor)
  (Development|PrintString "Destryoed" true true "(R=1.000000,G=0.000000,B=0.068582,A=1.000000)"))

(event Custom|Set%20Velocity
  (params (Initial%20Velocity :type Vector))
  (bind _sphere (Variables|Default|GetSphere))
  ;[0.15 0.15 0.15 0.5] Set Launch velocity and DYNAMIC Material Instance
  (Utilities|FlowControl|Sequence
    (:then_0
      (Variables|Default|SetVelocity Initial%20Velocity))
    (:then_1
      (bind _returnvalue (Rendering|Material|CreateDynamicMaterialInstance _sphere 0 (Rendering|Material|GetMaterial _sphere 0) "None" :!class /Script/Engine.PrimitiveComponent))
      (Variables|Default|SetDynMaterialInst _returnvalue))))

(event Custom|Add%20Force%20From%20Input
  (params (Force :type Vector))
  ;[0.15 0.15 0.15 0.5] Manual Input Force ( THRUSTERS )
  (Variables|Default|SetInput%20Force Force))

(event Custom|Won
  (bind _fx_orbit_trail (Variables|Default|GetFX_Orbit_Trail))
  ;[0.15 0.15 0.15 0.5] WON Cleanup
  (Variables|Default|SetisWon true)
  (Physics|SetSimulatePhysics (Variables|Default|GetSphere) false)
  (Widget|SetVisibility (Variables|Default|GetX%20Velocity%20Widget) "Collapsed")
  (Widget|SetVisibility (Variables|Default|GetY%20Velocity%20Widget) "Collapsed")
  (Components|Activation|Deactivate _fx_orbit_trail)
  (Rendering|ToggleVisibility _fx_orbit_trail false))

(event EventBeginPlay
  ;[0.15 0.15 0.15 0.5] Iniital Setup
  (Utilities|FlowControl|Sequence
    (:then_0
      (|SetVelocityWidgets))
    (:then_1
      (|LockPositionifRequired))
    (:then_2
      (|SetActiveStatusforOrbitTrail))
    (:then_3
      (bind _returnvalue (Actor|GetActorOfClass "/Game/Blueprints/BP_Simulator.BP_Simulator_C"))
      (Variables|Default|SetBP_Simulator _returnvalue)
      (bind _returnvalue_2 (Actor|GetActorOfClass "/Game/Blueprints/BP_Player.BP_Player_C"))
      (Variables|Default|SetBP_Player _returnvalue_2))
    (:then_4
      (Physics|SetPhysicsLinearVelocity (Variables|Default|GetSphere) (Variables|Default|GetInitialvelocity) false "None"))))

(event EventTick
  (params (DeltaSeconds :type Float%20%28single-precision%29))
  ;[0.15 0.15 0.15 0.5] TICK
  (if (not (Variables|Default|GetisWon))
    (Utilities|FlowControl|Sequence
      (:then_1
        (if (Variables|Default|GetShow%20Velocity)
          (|DrawDebugVelocityArrows DeltaSeconds)
          (|UpdateVelocityText)))
      (:then_2
        (if (|NotInsideCameraView)
          (CallFunction|DestroyBody)))
      (:then_3
        (Utilities|IsValid (Variables|Revolution|GetTargetActor)
          (:Is%20Valid
            (Revolution|RevolveAroundActor (* DeltaSeconds 5e+01))))))))

(event EventSetCurrentForceCPP
  (params (force :type Vector :default "0, 0, 0") (DeltaSeconds :type Float%20%28single-precision%29))
  (bind _sphere (Variables|Default|GetSphere))
  (if (not (Actor|ActorHasTag "avoid"))
    (bind _output_get (Variables|Default|SetNet%20Force force))
    (bind _output_get_2 (Variables|Default|SetVelocity (+ (* (/ _output_get (Physics|GetMass (Variables|Default|GetSphere))) DeltaSeconds) (Variables|Default|GetVelocity))))
    (Development|PrintString (Utilities|String|ToString(Vector) (* _output_get_2 DeltaSeconds)))
    (Transformation|SetWorldLocation _sphere (+ (* _output_get_2 DeltaSeconds) (Transformation|GetWorldLocation _sphere)) false false)
    (Transformation|SetActorRotation (Math|Rotator|MakeRotator 0.0 0.0 (.yaw (Math|Conversions|RotationFromXVector (Variables|Default|GetVelocity)))))))

(fn ConstructionScript
  (if (Utilities|String|Contains (Variables|Default|GetName) "Player")
    (Components|DestroyComponent (Variables|Default|GetGravity%20Well))
    (bind _returnvalue (Components|StaticMesh|SetStaticMesh (Variables|Default|GetSphere) "/Game/Rocket/rocket.rocket"))
    (Development|PrintString (Utilities|String|ToString(Boolean) _returnvalue))
    (else
      (Development|PrintString "No Player"))))

(fn RevolveAroundActor
  (params (AngleDeg :type Float%20%28single-precision%29))
  (Transformation|SetWorldLocation (Variables|Default|GetSphere) (+ (Math|Vector|RotateVectorAroundAxis (- (Transformation|GetActorLocation) (Transformation|GetActorLocation (Variables|Revolution|GetTargetActor))) AngleDeg "0.000000,0.000000,1.000000") (Transformation|GetActorLocation (Variables|Revolution|GetTargetActor))) false false))