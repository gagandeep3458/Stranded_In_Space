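; Player actor for a top-down gravity simulation: slingshot-launches the player's planet body, then thrusts it with directional input.
; Dragging spawns a BP_Body at the touch start and previews its path on a spline through the Simulator's C++ predictor.
; Release sets velocity from the drag vector, registers the body and starts the simulation, allowing only one launch.
; Directional inputs apply mass-scaled world-axis forces; BeginPlay derives world bounds from the orthographic camera.
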(event Input|EnhancedActionEvents|EnhancedInputActionIA_Forward
  (params (ActionValue :type Boolean) (ElapsedSeconds :type Float%20%28double-precision%29) (TriggeredSeconds :type Float%20%28double-precision%29) (InputAction :type Input%20Action%20Object%20Reference :default "/Game/Input/IA_Forward.IA_Forward"))
  (:Triggered
    (Default|AddForcefromInput (Variables|Default|GetPlayer%20Body) (* (Math|Vector|GetForwardVector "0, 0, 0") (Variables|Default|GetThrust%20Multiplier) (Class|BPCBody|GetMass (Variables|Default|GetPlayer%20Body)))))
  (:Canceled
    (Default|AddForcefromInput (Variables|Default|GetPlayer%20Body) "0, 0, 0" :!label _label))
  (:Completed
    (goto _label)))

(event Input|EnhancedActionEvents|EnhancedInputActionIA_Launch
  (params (ActionValue :type Vector%202D%20Structure) (ElapsedSeconds :type Float%20%28double-precision%29) (TriggeredSeconds :type Float%20%28double-precision%29) (InputAction :type Input%20Action%20Object%20Reference :default "/Game/Input/IA_Launch.IA_Launch"))
  (bind _simulator (Variables|Default|GetSimulator))
  (:Triggered
    (if (not (Variables|Default|GetPlayer%20Spawned))
      (if (not (Variables|Default|GetTouch%20Start%20Set))
        (Variables|Default|SetTouchStart (CallFunction|ToWorldSpaceCoord ActionValue))
        (Variables|Default|SetTouch%20Start%20Set true)
        (Rendering|SetVisibility (Variables|Default|GetNiagara) true true)
        (else
          (Variables|Default|SetTouchEnd (CallFunction|ToWorldSpaceCoord ActionValue))
          (Utilities|FlowControl|Sequence
            (:then_0
              ;[0.15 0.15 0.15 0.5] Spawn Body
              (Utilities|FlowControl|DoOnce false :!label _label
                (:Completed
                  (bind _returnvalue (Game|SpawnActorfromClass "/Game/Blueprints/BP_Body.BP_Body_C" (Math|Transform|MakeTransform (Math|Conversions|ToVector(Vector2D) (Variables|Default|GetTouchStart)) "0, 0, 0" (Math|Conversions|ToVector(Float) (Math|Float|MakeLiteralFloat 0.35))) "Undefined" "MultiplyWithRoot" 0 false true true "Player" 0 0))
                  (Variables|/Script/Engine.Actor|SetTags _returnvalue (Utilities|Array|MakeArray "Player"))
                  (bind _output_get (Variables|Default|SetPlayer%20Body _returnvalue))
                  (Class|PrimitiveComponent|SetMassOverrideinKg (Variables|/Script/Stranded_In_Space.BPC_Body|GetSphere _output_get) "None" 1e+03 true)
                  (Rendering|Material|SetMaterial (Variables|/Script/Stranded_In_Space.BPC_Body|GetSphere _output_get) 0 "/Game/Materials/Mat_Earth.Mat_Earth")
                  (Spline|ClearSplinePoints (Variables|Default|GetPathPredectionSpline) true))))
            (:then_1
              (Spline|ClearSplinePoints (Variables|Default|GetPathPredectionSpline) true)
              ;[0.15 0.15 0.15 0.5] Show Predective Path of Body
              (bind _returnvalue_2 (Class|BPCSimulator|GetPredectivePointwithCPP _simulator (Math|Conversions|ToVector(Vector2D) (Variables|Default|GetTouchStart)) (Math|Conversions|ToVector(Vector2D) (- (Variables|Default|GetTouchStart) (Variables|Default|GetTouchEnd))) 100 (Variables|Default|GetPlayer%20Body) (Variables|/Game/Blueprints/BP_Simulator.BP_Simulator_C|GetDelta%20Seconds _simulator) (Variables|/Game/Blueprints/BP_Simulator.BP_Simulator_C|GetBodies _simulator) (Variables|/Game/Blueprints/BP_Simulator.BP_Simulator_C|GetG_Constant _simulator)))
              (Spline|SetSplinePoints (Variables|Default|GetPathPredectionSpline) _returnvalue_2 "World" true)
              (Transformation|SetWorldRotation (Variables|/Script/Stranded_In_Space.BPC_Body|GetSphere (Variables|Default|GetPlayer%20Body)) (Math|Rotator|MakeRotator 0.0 0.0 (.yaw (Math|Conversions|RotationFromXVector (Math|Conversions|ToVector(Vector2D) (- (Variables|Default|GetTouchStart) (Variables|Default|GetTouchEnd)))))) false false)))))))
  (:Completed
    (if (not (Variables|Default|GetPlayer%20Spawned))
      (Rendering|SetVisibility (Variables|Default|GetNiagara) false true)
      (Spline|ClearSplinePoints (Variables|Default|GetPathPredectionSpline) true)
      ;[0.15 0.15 0.15 0.5] Initialize Spawned Body
      (Default|SetVelocity (Variables|Default|GetPlayer%20Body) (Math|Conversions|ToVector(Vector2D) (- (Variables|Default|GetTouchStart) (Variables|Default|GetTouchEnd))))
      (Default|AddBodytoSim (Variables|Default|GetSimulator) (Variables|Default|GetPlayer%20Body))
      (Variables|/Game/Blueprints/BP_Simulator.BP_Simulator_C|SetBegin%20Simulation (Variables|Default|GetSimulator) true)
      (Variables|Default|SetPlayer%20Spawned true)
      (|ResetLaunchValues_2)
      (goto _label Reset))))

(event Input|EnhancedActionEvents|EnhancedInputActionIA_Backward
  (params (ActionValue :type Boolean) (ElapsedSeconds :type Float%20%28double-precision%29) (TriggeredSeconds :type Float%20%28double-precision%29) (InputAction :type Input%20Action%20Object%20Reference :default "/Game/Input/IA_Backward.IA_Backward"))
  (:Triggered
    (Default|AddForcefromInput (Variables|Default|GetPlayer%20Body) (* (Math|Vector|GetForwardVector "0.000000,-180.000000,0.000000") (Variables|Default|GetThrust%20Multiplier) (Class|BPCBody|GetMass (Variables|Default|GetPlayer%20Body)))))
  (:Canceled
    (Default|AddForcefromInput (Variables|Default|GetPlayer%20Body) "0, 0, 0" :!label _label))
  (:Completed
    (goto _label)))

(event Input|EnhancedActionEvents|EnhancedInputActionIA_Left
  (params (ActionValue :type Boolean) (ElapsedSeconds :type Float%20%28double-precision%29) (TriggeredSeconds :type Float%20%28double-precision%29) (InputAction :type Input%20Action%20Object%20Reference :default "/Game/Input/IA_Left.IA_Left"))
  (:Triggered
    (Default|AddForcefromInput (Variables|Default|GetPlayer%20Body) (* (Math|Vector|GetForwardVector "0.000000,-90.000000,0.000000") (Variables|Default|GetThrust%20Multiplier) (Class|BPCBody|GetMass (Variables|Default|GetPlayer%20Body)))))
  (:Canceled
    (Default|AddForcefromInput (Variables|Default|GetPlayer%20Body) "0, 0, 0" :!label _label))
  (:Completed
    (goto _label)))

(event Input|EnhancedActionEvents|EnhancedInputActionIA_RIght
  (params (ActionValue :type Boolean) (ElapsedSeconds :type Float%20%28double-precision%29) (TriggeredSeconds :type Float%20%28double-precision%29) (InputAction :type Input%20Action%20Object%20Reference :default "/Game/Input/IA_RIght.IA_RIght"))
  (:Triggered
    (Default|AddForcefromInput (Variables|Default|GetPlayer%20Body) (* (Math|Vector|GetForwardVector "0.000000,90.000000,0.000000") (Variables|Default|GetThrust%20Multiplier) (Class|BPCBody|GetMass (Variables|Default|GetPlayer%20Body)))))
  (:Canceled
    (Default|AddForcefromInput (Variables|Default|GetPlayer%20Body) "0, 0, 0" :!label _label))
  (:Completed
    (goto _label)))

(event EventBeginPlay
  (Input|AddMappingContext (PlayerController|LocalPlayerSubsystems|GetEnhancedInputLocalPlayerSubsystem (Game|GetPlayerController 0)) "/Game/Input/IMC_Default.IMC_Default" 0 "(bIgnoreAllPressedKeysUntilRelease=True,bForceImmediately=False,bNotifyUserSettings=False)")
  (bind _returnvalue (Actor|GetActorOfClass "/Game/Blueprints/BP_Simulator.BP_Simulator_C"))
  (Variables|Default|SetSimulator _returnvalue)
  (bind _returnvalue_2 (Actor|GetActorOfClass "/Game/GravityGrid/Render_Target_Experiment/BP_GravityDrawer.BP_GravityDrawer_C"))
  (Variables|Default|SetBP%20Gravity%20Drawer _returnvalue_2)
  (|SetWorldBounds)
  (Spline|ClearSplinePoints (Variables|Default|GetPathPredectionSpline) true))

(fn ConstructionScript)

(fn ToWorldSpaceCoord
  (params (Vector%20in :type Vector%202D%20Structure))
  (bind (_x _y) (Math|Vector2D|BreakVector2D Vector%20in))
  (bind _returnvalue (Game|GetPlayerController 0))
  (bind _worldlocation (Class|PlayerController|DeprojectScreenPositiontoWorld _returnvalue _x _y))
  (bind (_x_2 _y_2) (Math|Vector|BreakVector _worldlocation))
  (return (Math|Vector2D|MakeVector2D _x_2 _y_2)))