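; BP_FinalWormhole is the goal actor that registers a win when a BP_Body hits its sphere.
; On the first such hit only, it removes the body from the BP_Simulator found at BeginPlay, prints a win message, then calls the body's Won and FadeBodyColor, passing itself to the latter.
; A separate one-shot FadeWormHole event uses a timeline to drive the Niagara effect's GlobalOpacity.
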(event OnComponentHit(Sphere)
  (params (HitComponent :type Primitive%20Component%20Object%20Reference) (OtherActor :type Actor%20Object%20Reference) (OtherComp :type Primitive%20Component%20Object%20Reference) (NormalImpulse :type Vector :default "0, 0, 0") (Hit :type Hit%20Result%20Structure%20%28by%20ref%29))
  (bind _asbp_body (Utilities|Casting|CastToBP_Body OtherActor))
  (Utilities|FlowControl|DoOnce false
    (:Completed
      (Utilities|FlowControl|Sequence
        (:then_0
          (Default|RemoveBody (Variables|Default|GetSimulator) _asbp_body)
          (Development|PrintString "You Won!"))
        (:then_1
          (Default|Won _asbp_body))
        (:then_2
          (Default|FadeBodyColor _asbp_body self))))))

(event Custom|FadeWormHole
  (Utilities|FlowControl|DoOnce false
    (:Completed
      (bind _value (Timeline|Timeline Play)
        (:Update
          (Niagara|SetNiagaraVariable(Float) (Variables|Default|GetNiagara) "GlobalOpacity" _value))))))

(event EventBeginPlay
  (bind _returnvalue (Actor|GetActorOfClass "/Game/Blueprints/BP_Simulator.BP_Simulator_C"))
  (Variables|Default|SetSimulator _returnvalue))

(fn ConstructionScript)