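; BP_GravityDrawer paints the UV footprint of every BP_Body into a canvas render target for a gravity grid experiment.
; On BeginPlay it gathers all bodies and creates a dynamic instance of a canvas material; AddBodyForDrawing registers further bodies.
; Each tick it clears the target to white, then draws the material full-size once per body, setting that body's hit UV and radius as parameters.
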(event Custom|Add%20Body%20For%20Drawing
  (params (Body :type BP%20Body%20Object%20Reference))
  (Utilities|Array|Add (Variables|Default|GetSpheres) Body))

(event EventBeginPlay
  (bind _outactors (Actor|GetAllActorsOfClass "/Game/Blueprints/BP_Body.BP_Body_C"))
  (Variables|Default|SetSpheres _outactors)
  (bind _output_get (Variables|Default|SetMatForCanvas "/Game/GravityGrid/Render_Target_Experiment/Mat_ForCanvas.Mat_ForCanvas"))
  (bind _returnvalue (Rendering|Material|CreateDynamicMaterialInstance _output_get "None" "None" :!class /Script/Engine.KismetMaterialLibrary))
  (Variables|Default|SetDynMatForCanvas _returnvalue))

(event EventTick
  (params (DeltaSeconds :type Float%20%28single-precision%29))
  (Rendering|ClearRenderTarget2D "/Game/GravityGrid/Render_Target_Experiment/NewCanvasRenderTarget2D.NewCanvasRenderTarget2D" "(R=1.000000,G=1.000000,B=1.000000,A=1.000000)")
  (bind (_canvas _size _context) (Rendering|BeginDrawCanvastoRenderTarget "/Game/GravityGrid/Render_Target_Experiment/NewCanvasRenderTarget2D.NewCanvasRenderTarget2D"))
  (for _array_element (Variables|Default|GetSpheres)
    (Rendering|Material|SetVectorParameterValue (Variables|Default|GetDynMatForCanvas) "UV Coord" (Math|Conversions|ToLinearColor(Vector) (Math|Vector|MakeVector (.x (Variables|/Game/Blueprints/BP_Body.BP_Body_C|GetHitLocationUV _array_element)) (.y (Variables|/Game/Blueprints/BP_Body.BP_Body_C|GetHitLocationUV _array_element)) 0.0)) :!class /Script/Engine.MaterialInstanceDynamic)
    (Rendering|Material|SetScalarParameterValue (Variables|Default|GetDynMatForCanvas) "UV Radius" (Variables|/Game/Blueprints/BP_Body.BP_Body_C|GetRadiusInUV _array_element) :!class /Script/Engine.MaterialInstanceDynamic)
    (Canvas|DrawMaterial :self _canvas :RenderMaterial (Variables|Default|GetDynMatForCanvas) :ScreenSize (Math|Vector2D|MakeVector2D 1024.0 1024.0) :CoordinateSize "(X=1.000000,Y=1.000000)" :PivotPoint "(X=0.500000,Y=0.500000)"))
  (Rendering|EndDrawCanvastoRenderTarget _context))

(fn ConstructionScript)