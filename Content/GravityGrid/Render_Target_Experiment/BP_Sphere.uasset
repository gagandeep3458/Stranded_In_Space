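; BP_Sphere is a render-target experiment actor that orbits the world origin and computes its circular footprint in a BP_Plane's UV space.
; BeginPlay finds the plane and derives RadiusInUV by normalizing the sphere's X extent against the plane's scaled bounds.
; Each Tick rotates the actor about world Z, then runs a debug-drawn complex downward trace.
; FindCollisionUV turns the hit into HitLocationUV, the circle's center.
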(event EventBeginPlay
  (bind _sphere (Variables|Default|GetSphere))
  (bind _max (Components|StaticMesh|GetLocalBounds _sphere))
  (bind _returnvalue (Transformation|GetWorldScale _sphere))
  (bind _returnvalue_2 (Transformation|GetWorldLocation _sphere))
  (bind _returnvalue_3 (* _returnvalue _max))
  (bind _returnvalue_4 (Actor|GetActorOfClass "/Game/GravityGrid/Render_Target_Experiment/BP_Plane.BP_Plane_C"))
  (Variables|Default|SetBP_Plane _returnvalue_4)
  (bind _output_get (Variables|Default|SetRadiusInUV (.x (/ (- (/ (- (+ _returnvalue_2 _returnvalue_3) (- (Transformation|GetWorldLocation (Variables|/Game/GravityGrid/Render_Target_Experiment/BP_Plane.BP_Plane_C|GetPlane (Variables|Default|GetBP_Plane))) (* (Transformation|GetWorldScale (Variables|/Game/GravityGrid/Render_Target_Experiment/BP_Plane.BP_Plane_C|GetPlane (Variables|Default|GetBP_Plane))) (.Max (Components|StaticMesh|GetLocalBounds (Variables|/Game/GravityGrid/Render_Target_Experiment/BP_Plane.BP_Plane_C|GetPlane (Variables|Default|GetBP_Plane))))))) (- (+ (Transformation|GetWorldLocation (Variables|/Game/GravityGrid/Render_Target_Experiment/BP_Plane.BP_Plane_C|GetPlane (Variables|Default|GetBP_Plane))) (* (Transformation|GetWorldScale (Variables|/Game/GravityGrid/Render_Target_Experiment/BP_Plane.BP_Plane_C|GetPlane (Variables|Default|GetBP_Plane))) (.Max (Components|StaticMesh|GetLocalBounds (Variables|/Game/GravityGrid/Render_Target_Experiment/BP_Plane.BP_Plane_C|GetPlane (Variables|Default|GetBP_Plane)))))) (- (Transformation|GetWorldLocation (Variables|/Game/GravityGrid/Render_Target_Experiment/BP_Plane.BP_Plane_C|GetPlane (Variables|Default|GetBP_Plane))) (* (Transformation|GetWorldScale (Variables|/Game/GravityGrid/Render_Target_Experiment/BP_Plane.BP_Plane_C|GetPlane (Variables|Default|GetBP_Plane))) (.Max (Components|StaticMesh|GetLocalBounds (Variables|/Game/GravityGrid/Render_Target_Experiment/BP_Plane.BP_Plane_C|GetPlane (Variables|Default|GetBP_Plane)))))))) (/ (- (- _returnvalue_2 _returnvalue_3) (- (Transformation|GetWorldLocation (Variables|/Game/GravityGrid/Render_Target_Experiment/BP_Plane.BP_Plane_C|GetPlane (Variables|Default|GetBP_Plane))) (* (Transformation|GetWorldScale (Variables|/Game/GravityGrid/Render_Target_Experiment/BP_Plane.BP_Plane_C|GetPlane (Variables|Default|GetBP_Plane))) (.Max (Components|StaticMesh|GetLocalBounds (Variables|/Game/GravityGrid/Render_Target_Experiment/BP_Plane.BP_Plane_C|GetPlane (Variables|Default|GetBP_Plane))))))) (- (+ (Transformation|GetWorldLocation (Variables|/Game/GravityGrid/Render_Target_Experiment/BP_Plane.BP_Plane_C|GetPlane (Variables|Default|GetBP_Plane))) (* (Transformation|GetWorldScale (Variables|/Game/GravityGrid/Render_Target_Experiment/BP_Plane.BP_Plane_C|GetPlane (Variables|Default|GetBP_Plane))) (.Max (Components|StaticMesh|GetLocalBounds (Variables|/Game/GravityGrid/Render_Target_Experiment/BP_Plane.BP_Plane_C|GetPlane (Variables|Default|GetBP_Plane)))))) (- (Transformation|GetWorldLocation (Variables|/Game/GravityGrid/Render_Target_Experiment/BP_Plane.BP_Plane_C|GetPlane (Variables|Default|GetBP_Plane))) (* (Transformation|GetWorldScale (Variables|/Game/GravityGrid/Render_Target_Experiment/BP_Plane.BP_Plane_C|GetPlane (Variables|Default|GetBP_Plane))) (.Max (Components|StaticMesh|GetLocalBounds (Variables|/Game/GravityGrid/Render_Target_Experiment/BP_Plane.BP_Plane_C|GetPlane (Variables|Default|GetBP_Plane))))))))) 2.0))))
  (Development|PrintString (Utilities|String|ToString(Float) _output_get)))

(event EventTick
  (params (DeltaSeconds :type Float%20%28single-precision%29))
  (bind _returnvalue (* DeltaSeconds 3e+01))
  (bind _defaultsceneroot (Variables|Default|GetDefaultSceneRoot))
  (bind _returnvalue_2 (Transformation|GetWorldLocation _defaultsceneroot))
  (bind _returnvalue_3 (Math|Vector|RotateVectorAroundAxis _returnvalue_2 _returnvalue "0.000000,0.000000,1.000000"))
  (Transformation|SetWorldLocation _defaultsceneroot _returnvalue_3 false false)
  (bind _outhit (Collision|LineTraceByChannel _returnvalue_3 (+ _returnvalue_3 "0.000000,0.000000,-500.000000") "TraceTypeQuery1" true 0 "ForOneFrame"))
  (Variables|Default|SetHit%20Location%20UV (.UV (Class|GameplayStatics|FindCollisionUV _outhit))))

(fn ConstructionScript)